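; Couple manager for the cupid shooter game that pairs and separates BP_NPCs and tracks healthy and toxic couple counts.
; A two-way map, seeded from each NPC's preset partner with all couples counted toxic, gives lookup from either side.
; CoupleAssign holds the first suitor until a second arrives, then links them, judging health by matching Color.
; Pairing and Breakup trigger NPC flight, update outlines and send counts to the BP_CupidShooter game mode.
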(event `self.ReceiveBeginPlay`
  (bind _outactors (`GameplayStatics.GetAllActorsOfClass` "/Game/Mall/NPC/BP_NPC.BP_NPC_C"))
  (for _array_element _outactors
    (`BlueprintMapLibrary.Map_Add` (`self.Couples`) _array_element (`/Game/Mall/NPC/BP_NPC.PartnerNPC` _array_element)))
  (set `self.NumOfToxicCouples` (/ (`BlueprintMapLibrary.Map_Length` (`self.Couples`)) 2)))

(event `self.ReceiveTick`
  (params (DeltaSeconds :type "Float (single-precision)")))

(fn `breakup`
  (params (Suitor :type "/Game/Mall/NPC/BP_NPC Object Reference"))
  (set `self.Suitor` Suitor)
  (if (`BlueprintMapLibrary.Map_Contains` (`self.Couples`) (`self.Suitor`))
    (set `self.ex` (`BlueprintMapLibrary.Map_Find` (`self.Couples`) (`self.Suitor`)))
    (`BlueprintMapLibrary.Map_Remove` (`self.Couples`) (`self.Suitor`))
    (`BlueprintMapLibrary.Map_Remove` (`self.Couples`) (`self.ex`))
    (`/Game/Mall/NPC/BP_NPC.flyAway` (`self.ex`) (`self.K2_GetActorLocation` (`self.Suitor`)))
    (`/Game/Mall/NPC/BP_NPC.flyAway` (`self.Suitor`) (`self.K2_GetActorLocation` (`self.ex`)))
    (if (`/Game/Mall/NPC/BP_NPC.HealthyRelationship?` (`self.Suitor`))
      (bind _result (`/Engine/EditorBlueprintResources/StandardMacros.DecrementInt` (`self.NumOfHealthyCouples`))
        (:`  `
          (bind _asbp_cupid_shooter (cast `/Game/Mall/BP_CupidShooter` (`GameplayStatics.GetGameMode`)))
          ; change outline
          (bind _output_get (set `/Game/Mall/NPC/BP_NPC.HealthyRelationship?` false (`self.ex`)))
          (set `/Game/Mall/NPC/BP_NPC.HealthyRelationship?` _output_get (`self.Suitor`))
          (bind _output_get_2 (set `/Game/Mall/NPC/BP_NPC.InRelationShip?` false (`self.ex`)))
          (set `/Game/Mall/NPC/BP_NPC.InRelationShip?` _output_get_2 (`self.Suitor`))
          (`/Game/Mall/NPC/BP_NPC.SetOutline` (`self.ex`))
          (`/Game/Mall/NPC/BP_NPC.SetOutline` (`self.Suitor`))
          (`/Game/Mall/BP_CupidShooter.Set Healthy Couple` _asbp_cupid_shooter _result)))
      (else
        (bind _result_2 (`/Engine/EditorBlueprintResources/StandardMacros.DecrementInt` (`self.NumOfToxicCouples`))
          (:`  `
            (bind _asbp_cupid_shooter_2 (cast `/Game/Mall/BP_CupidShooter` (`GameplayStatics.GetGameMode`)))
            ; change outline
            (bind _output_get_3 (set `/Game/Mall/NPC/BP_NPC.HealthyRelationship?` false (`self.ex`)))
            (set `/Game/Mall/NPC/BP_NPC.HealthyRelationship?` _output_get_3 (`self.Suitor`))
            (bind _output_get_4 (set `/Game/Mall/NPC/BP_NPC.InRelationShip?` false (`self.ex`)))
            (set `/Game/Mall/NPC/BP_NPC.InRelationShip?` _output_get_4 (`self.Suitor`))
            (`/Game/Mall/NPC/BP_NPC.SetOutline` (`self.ex`))
            (`/Game/Mall/NPC/BP_NPC.SetOutline` (`self.Suitor`))
            (`/Game/Mall/BP_CupidShooter.Set Toxic Couple` _asbp_cupid_shooter_2 _result_2)))))))

(fn `couple_assign`
  (params (Suitor :type "/Game/Mall/NPC/BP_NPC Object Reference"))
  (set `self.Suitor` Suitor)
  ; sees if suitor has a partner
  (if (`BlueprintMapLibrary.Map_Contains` (`self.Couples`) (`self.Suitor`))
    (`KismetSystemLibrary.PrintString` "no polyamorty allowed")
    (else
      ; checks to see if you already picked one person to be in couple
      (if (`KismetSystemLibrary.IsValid` (`self.WaitingPawn`))
        ; no self love allowed
        (if (== (`self.Suitor`) (`self.WaitingPawn`))
          (`KismetSystemLibrary.PrintString` "no self love")
          (else
            (`KismetSystemLibrary.PrintString` "it now has soemthing" false)
            ; adds couple to map, in both ways so either person can be found later, only adds matching couples can be changed
            (`BlueprintMapLibrary.Map_Add` (`self.Couples`) (`self.Suitor`) (`self.WaitingPawn`))
            (`BlueprintMapLibrary.Map_Add` (`self.Couples`) (`self.WaitingPawn`) (`self.Suitor`))
            (set `/Game/Mall/NPC/BP_NPC.InRelationShip?` true (`self.WaitingPawn`))
            (set `/Game/Mall/NPC/BP_NPC.InRelationShip?` true (`self.Suitor`))
            (`/Game/Mall/NPC/BP_NPC.FlytoThem` (`self.WaitingPawn`) (`self.K2_GetActorLocation` (`self.Suitor`)))
            (if (`|EnumEquality` (`/Game/Mall/NPC/BP_NPC.Color` (`self.Suitor`)) (`/Game/Mall/NPC/BP_NPC.Color` (`self.WaitingPawn`)))
              (bind _output_get (set `/Game/Mall/NPC/BP_NPC.HealthyRelationship?` true (`self.WaitingPawn`)))
              (set `/Game/Mall/NPC/BP_NPC.HealthyRelationship?` _output_get (`self.Suitor`))
              ; change outline
              (bind _asbp_npc (cast `/Game/Mall/NPC/BP_NPC` (`self.WaitingPawn`)))
              (`/Game/Mall/NPC/BP_NPC.SetOutline` _asbp_npc)
              (bind _asbp_npc_2 (cast `/Game/Mall/NPC/BP_NPC` (`self.Suitor`)))
              (`/Game/Mall/NPC/BP_NPC.SetOutline` _asbp_npc_2)
              (set `self.WaitingPawn` null)
              ; testing print
              (bind _asbp_cupid_shooter (cast `/Game/Mall/BP_CupidShooter` (`GameplayStatics.GetGameMode`)))
              (bind _result (`/Engine/EditorBlueprintResources/StandardMacros.IncrementInt` (`self.NumOfHealthyCouples`))
                (:`  `
                  (`/Game/Mall/BP_CupidShooter.Set Healthy Couple` _asbp_cupid_shooter _result)))
              (else
                (`KismetSystemLibrary.PrintString` "dont match! ")
                (bind _output_get_2 (set `/Game/Mall/NPC/BP_NPC.HealthyRelationship?` false (`self.WaitingPawn`)))
                (set `/Game/Mall/NPC/BP_NPC.HealthyRelationship?` _output_get_2 (`self.Suitor`))
                (bind _asbp_npc_3 (cast `/Game/Mall/NPC/BP_NPC` (`self.WaitingPawn`)))
                (`/Game/Mall/NPC/BP_NPC.SetOutline` _asbp_npc_3)
                (bind _asbp_npc_4 (cast `/Game/Mall/NPC/BP_NPC` (`self.Suitor`)))
                (`/Game/Mall/NPC/BP_NPC.SetOutline` _asbp_npc_4)
                (set `self.WaitingPawn` null)
                (bind _asbp_cupid_shooter_2 (cast `/Game/Mall/BP_CupidShooter` (`GameplayStatics.GetGameMode`)))
                (bind _result_2 (`/Engine/EditorBlueprintResources/StandardMacros.IncrementInt` (`self.NumOfToxicCouples`))
                  (:`  `
                    (`/Game/Mall/BP_CupidShooter.Set Toxic Couple` _asbp_cupid_shooter_2 _result_2)))))))
        (else
          (`KismetSystemLibrary.PrintString` "pawn was empty when i checked" false)
          ; assigns person on standby
          (set `self.WaitingPawn` (`self.Suitor`)))))))

(fn `UserConstructionScript`)