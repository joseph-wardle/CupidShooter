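; Mall NPC actor whose cube visually shows its color and relationship status.
; The construction script applies a material from the Color enum and an overlay outline for no, healthy or unhealthy relationship.
; FlytoThem instantly moves the NPC to a fixed distance short of a destination, along the line from its current position, then fires a debug print event.
; A Timeline and a face-the-player rotation are left unwired.
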(event `self.ReceiveTick`
  (params (DeltaSeconds :type "Float (single-precision)")))

(event `peepeepoopoo`
  (`KismetSystemLibrary.PrintString` "peepee"))

(fn `FlytoThem`
  (params (destination :type "Vector Structure"))
  (`self.K2_SetActorLocation` (- destination (* (`KismetMathLibrary.Normal` (- destination (`self.K2_GetActorLocation`))) (600.0 600.0 600.0))))
  (`self.peepeepoopoo`))

(fn `SetColor`
  (bind _cube (`self.Cube`))
  (switch `/Game/Mall/NPC/E_PairTypes` (`self.Color`)
    (:`NewEnumerator0`
      (`PrimitiveComponent.SetMaterial` _cube 0 "/Game/Mall/NPC/M_Red.M_Red"))
    (:`NewEnumerator1`
      (`PrimitiveComponent.SetMaterial` _cube 0 "/Game/Mall/NPC/M_Green.M_Green"))
    (:`NewEnumerator2`
      (`PrimitiveComponent.SetMaterial` _cube 0 "/Game/Mall/NPC/M_Blue.M_Blue"))
    (:`NewEnumerator3`
      (`PrimitiveComponent.SetMaterial` _cube 0 "/Game/Mall/NPC/M_Yellow.M_Yellow"))))

(fn `SetOutline`
  (if (`self.InRelationShip?`)
    (if (`self.HealthyRelationship?`)
      (`MeshComponent.SetOverlayMaterial` (`self.Cube`) "/Game/Mall/NPC/Outline_Healthy.Outline_Healthy")
      (else
        (`MeshComponent.SetOverlayMaterial` (`self.Cube`) "/Game/Mall/NPC/Outline_Unhealthy.Outline_Unhealthy")))
    (else
      (`MeshComponent.SetOverlayMaterial` (`self.Cube`) "/Game/Mall/NPC/Outline_noRelationship.Outline_noRelationship"))))

(fn `UserConstructionScript`
  (`self.SetColor`)
  (`self.SetOutline`))