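; BP_CupidShooter manages the HUD and level reset for the mall Cupid shooter game, which tallies healthy and toxic couples.
; On BeginPlay it creates WB_PlayerWidget and adds it to the viewport.
; Couple events pass their counts to the widget, and the healthy-couple event also copies the widget's EndGame value into GameEnded.
; Reset reopens L_Mall.
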(event `self.ReceiveBeginPlay`
  (bind _returnvalue (`|CreateWidget` "/Game/Mall/WB_PlayerWidget.WB_PlayerWidget_C"))
  (bind _output_get (set `self.HUD` _returnvalue))
  (`UserWidget.AddToViewport` _returnvalue 0)
  (`UserWidget.AddToViewport` _output_get 0))

(event `Reset`
  (`GameplayStatics.OpenLevelBySoftObjectPtr` "/Game/Mall/L_Mall.L_Mall"))

(event `Set Healthy Couple`
  (params (NumGoodCouples :type Integer))
  (bind _aswb_player_widget (cast `/Game/Mall/WB_PlayerWidget` (`self.HUD`)))
  (`/Game/Mall/WB_PlayerWidget.SetGoodCouples` _aswb_player_widget NumGoodCouples)
  (set `self.GameEnded` (`/Game/Mall/WB_PlayerWidget.EndGame` _aswb_player_widget)))

(event `Set Toxic Couple`
  (params (NumBadCouples :type Integer))
  (bind _aswb_player_widget (cast `/Game/Mall/WB_PlayerWidget` (`self.HUD`)))
  (`/Game/Mall/WB_PlayerWidget.SetBadCouples` _aswb_player_widget NumBadCouples))

(fn `UserConstructionScript`)