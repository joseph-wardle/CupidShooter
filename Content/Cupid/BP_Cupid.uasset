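; BP_Cupid is the first-person or third-person player Cupid character, who pairs up and breaks up NPCs.
; Love-gun and break-up inputs line trace from the camera, filter hits by "BP_NPC" name, and pass the NPC to BP_CoupleManagerGS.
; Enhanced Input also drives movement, a directional dash, limited multi-jumps refilled on landing, and a slide/ground pound.
; These moves combine LaunchCharacter with gravity, walk-speed or capsule-size changes.
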(event `self.ReceiveBeginPlay`
  (bind _returnvalue (`GameplayStatics.GetPlayerController` 0))
  (`EnhancedInputSubsystemInterface.AddMappingContext` (pcsubsystem `EnhancedInputLocalPlayerSubsystem` _returnvalue) "/Game/Cupid/IMC_Controls.IMC_Controls" 0 (struct))
  (`Controller.Possess` _returnvalue null))

(event `self.ReceiveTick`
  (params (DeltaSeconds :type "Float (single-precision)")))

(event `InputVectorAxis|Mouse2D`
  (params (AxisValue :type "Vector Structure"))
  ; Looking Around
  (`self.AddControllerYawInput` AxisValue_X)
  (`self.AddControllerPitchInput` (* AxisValue_Y -1.0)))

(event `EnhancedInput|/Game/Cupid/IA_LoveGun`
  (params (ActionValue :type Boolean) (ElapsedSeconds :type "Float (double-precision)") (TriggeredSeconds :type "Float (double-precision)") (InputAction :type "InputAction Object Reference" :default "/Game/Cupid/IA_LoveGun.IA_LoveGun"))
  (bind _playercameramanager (`PlayerController.PlayerCameraManager` (`GameplayStatics.GetPlayerController` 0)))
  (bind _returnvalue (`PlayerCameraManager.GetCameraLocation` _playercameramanager))
  (:`Started`
    (bind _outhit (`KismetSystemLibrary.LineTraceSingle` :`Start` _returnvalue :`End` (+ _returnvalue (* (`KismetMathLibrary.GetForwardVector` (`PlayerCameraManager.GetCameraRotation` _playercameramanager)) 50000)) :`TraceChannel` "TraceTypeQuery2" :`DrawDebugType` "ForOneFrame"))
    (bind (_bblockinghit _binitialoverlap _time _distance _location _impactpoint _normal _impactnormal _physmat _hitactor) (`GameplayStatics.BreakHitResult` _outhit))
    (if (== (`KismetStringLibrary.FindSubstring` (`KismetSystemLibrary.GetDisplayName` _hitactor) "BP_NPC") 0)
      (bind _asbp_npc (cast `/Game/Mall/NPC/BP_NPC` _hitactor))
      (bind _asbp_couple_manager_gs (cast `/Game/Mall/BP_CoupleManagerGS` (`GameplayStatics.GetGameState`)))
      (`/Game/Mall/BP_CoupleManagerGS.couple_assign` _asbp_couple_manager_gs _asbp_npc))))

(event `EnhancedInput|/Game/Cupid/IA_CupidMove`
  (params (ActionValue :type "Vector2D Structure") (ElapsedSeconds :type "Float (double-precision)") (TriggeredSeconds :type "Float (double-precision)") (InputAction :type "InputAction Object Reference" :default "/Game/Cupid/IA_CupidMove.IA_CupidMove"))
  (bind (_returnvalue_roll _returnvalue_pitch _returnvalue_yaw) (`KismetMathLibrary.BreakRotator` (`self.GetControlRotation`)))
  (bind _returnvalue (`KismetMathLibrary.MakeRotator` 0.0 0.0 _returnvalue_yaw))
  ; WASD Movements
  (:`Triggered`
    (`self.AddMovementInput` (+ (* ActionValue_X (`KismetMathLibrary.GetForwardVector` _returnvalue)) (* ActionValue_Y (`KismetMathLibrary.GetRightVector` _returnvalue))))))

(event `EnhancedInput|/Game/Cupid/IA_BreakUp`
  (params (ActionValue :type Boolean) (ElapsedSeconds :type "Float (double-precision)") (TriggeredSeconds :type "Float (double-precision)") (InputAction :type "InputAction Object Reference" :default "/Game/Cupid/IA_BreakUp.IA_BreakUp"))
  (bind _playercameramanager (`PlayerController.PlayerCameraManager` (`GameplayStatics.GetPlayerController` 0)))
  (bind _returnvalue (`PlayerCameraManager.GetCameraLocation` _playercameramanager))
  (:`Triggered`
    (bind _outhit (`KismetSystemLibrary.LineTraceSingle` :`Start` _returnvalue :`End` (+ _returnvalue (* (`KismetMathLibrary.GetForwardVector` (`PlayerCameraManager.GetCameraRotation` _playercameramanager)) 50000)) :`TraceChannel` "TraceTypeQuery2" :`DrawDebugType` "ForOneFrame"))
    (bind (_bblockinghit _binitialoverlap _time _distance _location _impactpoint _normal _impactnormal _physmat _hitactor) (`GameplayStatics.BreakHitResult` _outhit))
    (if (== (`KismetStringLibrary.FindSubstring` (`KismetSystemLibrary.GetDisplayName` _hitactor) "BP_NPC") 0)
      (bind _asbp_npc (cast `/Game/Mall/NPC/BP_NPC` _hitactor))
      (bind _asbp_couple_manager_gs (cast `/Game/Mall/BP_CoupleManagerGS` (`GameplayStatics.GetGameState`)))
      (`/Game/Mall/BP_CoupleManagerGS.breakup` _asbp_couple_manager_gs _asbp_npc))))

(event `EnhancedInput|/Game/Cupid/IA_SlideGroundPound`
  (params (ActionValue :type Boolean) (ElapsedSeconds :type "Float (double-precision)") (TriggeredSeconds :type "Float (double-precision)") (InputAction :type "InputAction Object Reference" :default "/Game/Cupid/IA_SlideGroundPound.IA_SlideGroundPound"))
  (bind (_returnvalue_roll _returnvalue_pitch _returnvalue_yaw) (`KismetMathLibrary.BreakRotator` (`self.GetControlRotation`)))
  ; Slide
  (:`Triggered`
    ;; Lower player to the ground and speed them up
    (if (`self.Sliding`)
      (`CapsuleComponent.SetCapsuleSize` (`self.CapsuleComponent`) 15.0 44.0 true)
      (set `CharacterMovementComponent.GravityScale` 1000.0 (`self.CharacterMovement`))
      (`self.LaunchCharacter` (+ (* (`self.GetLastMovementInputVector`) 2000.0) (* (`KismetMathLibrary.GetForwardVector` (`KismetMathLibrary.MakeRotator` 0.0 0.0 _returnvalue_yaw)) 10000.0)) true)))
  (:`Started`
    ;; Make put them on the ground
    (`self.LaunchCharacter` (0.0 0.0 -5000.0) true true)
    (set `CharacterMovementComponent.GravityScale` 1000.0 (`self.CharacterMovement`))
    (set `self.Sliding` true))
  (:`Completed`
    ;; Reset the player height and gravity
    (`CapsuleComponent.SetCapsuleSize` (`self.CapsuleComponent`) 34.0 200.0 true)
    (set `CharacterMovementComponent.GravityScale` 5.0 (`self.CharacterMovement`))
    (set `self.ExitingSlide` true)
    (`KismetSystemLibrary.Delay` 1.0)
    (set `self.ExitingSlide` false)))

(event `EnhancedInput|/Game/Cupid/IA_Dash`
  (params (ActionValue :type Boolean) (ElapsedSeconds :type "Float (double-precision)") (TriggeredSeconds :type "Float (double-precision)") (InputAction :type "InputAction Object Reference" :default "/Game/Cupid/IA_Dash.IA_Dash"))
  (bind (_returnvalue_x _returnvalue_y _returnvalue_z) (`KismetMathLibrary.BreakVector` (`KismetMathLibrary.GetForwardVector` (`self.GetControlRotation`))))
  ; Dash
  (:`Started`
    (`self.LaunchCharacter` (`KismetMathLibrary.MakeVector` (* _returnvalue_x 20000.0) (* _returnvalue_y 20000.0) (* _returnvalue_z 5000.0)) true)))

(event `EnhancedInput|/Game/Cupid/IA_CupidJump`
  (params (ActionValue :type Boolean) (ElapsedSeconds :type "Float (double-precision)") (TriggeredSeconds :type "Float (double-precision)") (InputAction :type "InputAction Object Reference" :default "/Game/Cupid/IA_CupidJump.IA_CupidJump"))
  ; Jumping Logic
  (:`Started`
    (if (!= (`self.AmountOfJumps`) 0)
      (set `self.Sliding` false)
      (set `CharacterMovementComponent.GravityScale` 5.0 (`self.CharacterMovement`))
      (`self.LaunchCharacter` (+ (* (`self.GetLastMovementInputVector`) 10000.0) (0.0 0.0 4000.0)) true true)
      (set `self.AmountOfJumps` (- (`self.AmountOfJumps`) 1))
      (set `self.IsJumping` true)
      (set `CharacterMovementComponent.MaxWalkSpeed` 5000.0 (`self.CharacterMovement`))))
  (:`Completed`
    (set `CharacterMovementComponent.GravityScale` 10.0 (`self.CharacterMovement`))))

(event `self.OnLanded`
  (params (Hit :type "HitResult Structure (by ref)"))
  ; Jumping Logic
  (set `CharacterMovementComponent.GravityScale` 5.0 (`self.CharacterMovement`))
  (set `self.AmountOfJumps` 2)
  (set `self.IsJumping` false)
  (set `CharacterMovementComponent.MaxWalkSpeed` 2500.0 (`self.CharacterMovement`)))

(fn `UserConstructionScript`)